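; A primary attack ability Blueprint that cycles through an array of montages, forming a combo chain.
; Each activation wraps the index if needed, plays that montage, then immediately advances the index.
; A montage notify marks the ability interruptible on the AbilitySystemComponent.
; Interruption preserves the index so the chain continues, while blending out resets it to the first montage.
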(event `self.OnActivateAbility`
  (`self.HandleMontageIndex`)
  (`|PlayMontage` (`self.CharacterMeshComponent`) (`|GetArrayItem` (`self.MontagetoPlay`) (`self.MontageIndex`)) (`self.MontagePlayRate`) (`self.MontageStartingPosition`)
    (:`then`
      (`/Engine/EditorBlueprintResources/StandardMacros.IncrementInt` (`self.MontageIndex`)))
    (:`OnBlendOut`
      (`self.PrintDebugMessage` "End")
      (`self.OnEndAbility` false))
    (:`OnInterrupted`
      (`self.PrintDebugMessage` "Interrupted")
      (`self.OnEndAbility` true))
    (:`OnNotifyBegin`
      (set `/Game/Framework/AbilitySystem/ARPGAbilitySystemComponent_BP.CanInterruptAbility` true (`self.AbilitySystemComponent`)))))

(event `self.OnEndAbility`
  (params (WasAbilityInterrupted :type Boolean))
  (`parent.OnEndAbility` false)
  (if (not WasAbilityInterrupted)
    (set `self.MontageIndex` 0)))

(fn `CanActivateAbility`
  (returns (CanActivateAbility :type Boolean))
  (return true))

(fn `HandleMontageIndex`
  (if (== (`self.MontageIndex`) (`KismetArrayLibrary.Array_Length` (`self.MontagetoPlay`)))
    (set `self.MontageIndex` 0)))