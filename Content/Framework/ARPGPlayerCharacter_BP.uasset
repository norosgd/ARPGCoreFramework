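; ARPGPlayerCharacter_BP is the player character for an action RPG, handling movement, camera look and jumping through Enhanced Input.
; On BeginPlay it adds the base input mapping context to its player controller's subsystem.
; Movement follows control-rotation forward and right vectors, camera input feeds controller yaw and pitch, and jump starts and stops with the button.
; Leftover global time dilation nodes for slow motion are unconnected and never run.
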(event `self.ReceiveBeginPlay`
  (bind _asplayer_controller (cast `PlayerController` (`self.GetController`)))
  (`/Engine/EditorBlueprintResources/StandardMacros.IsValid` _asplayer_controller
    (:`Is Valid`
      (`EnhancedInputSubsystemInterface.AddMappingContext` (pcsubsystem `EnhancedInputLocalPlayerSubsystem` _asplayer_controller) "/Game/EnhancedInput/IMC_ARPGBaseInputContext.IMC_ARPGBaseInputContext" 0 (struct)))))

(event `EnhancedInput|/Game/EnhancedInput/IA_Movement`
  (params (ActionValue :type "Vector2D Structure") (ElapsedSeconds :type "Float (double-precision)") (TriggeredSeconds :type "Float (double-precision)") (InputAction :type "InputAction Object Reference" :default "/Game/EnhancedInput/IA_Movement.IA_Movement"))
  (bind _returnvalue (`self.GetControlRotation`))
  (bind (_x _y) (`KismetMathLibrary.BreakVector2D` ActionValue))
  (:`Triggered`
    (`self.AddMovementInput` (`KismetMathLibrary.GetForwardVector` _returnvalue) _y)
    (`self.AddMovementInput` (`KismetMathLibrary.GetRightVector` _returnvalue) _x)))

(event `EnhancedInput|/Game/EnhancedInput/IA_Camera`
  (params (ActionValue :type "Vector2D Structure") (ElapsedSeconds :type "Float (double-precision)") (TriggeredSeconds :type "Float (double-precision)") (InputAction :type "InputAction Object Reference" :default "/Game/EnhancedInput/IA_Camera.IA_Camera"))
  (bind (_x _y) (`KismetMathLibrary.BreakVector2D` ActionValue))
  (:`Triggered`
    (`self.AddControllerYawInput` _x)
    (`self.AddControllerPitchInput` _y)))

(event `EnhancedInput|/Game/EnhancedInput/IA_Jump`
  (params (ActionValue :type Boolean) (ElapsedSeconds :type "Float (double-precision)") (TriggeredSeconds :type "Float (double-precision)") (InputAction :type "InputAction Object Reference" :default "/Game/EnhancedInput/IA_Jump.IA_Jump"))
  (:`Started`
    (`self.Jump`))
  (:`Completed`
    (`self.StopJumping`)))

(fn `UserConstructionScript`
  (`parent.UserConstructionScript`))