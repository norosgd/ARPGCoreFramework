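; Base ability class for the ARPG ability system, defining the shared interface and setup for abilities.
; InitializeAbility caches the owner character, ability system component and character mesh, then fires OnInitializeAbility.
; The initialize, activate and end events are empty hooks, and CanActivateAbility returns false by default.
; PrintDebugMessage prints a string only when debug mode is on.
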(event `OnInitializeAbility`)

(event `OnActivateAbility`)

(event `OnEndAbility`)

(fn `CanActivateAbility`
  (returns (CanActivateAbility :type Boolean))
  (return false))

(fn `InitializeAbility`
  (params (OwnerCharacter :type "/Game/Framework/ARPGBaseCharacter_BP Object Reference") (AbilitySystemComponent :type "/Game/Framework/AbilitySystem/ARPGAbilitySystemComponent_BP Object Reference"))
  (bind _output_get (set `self.OwnerCharacter` OwnerCharacter))
  (set `self.AbilitySystemComponent` AbilitySystemComponent)
  (set `self.CharacterMeshComponent` (`Character.Mesh` _output_get))
  (`self.OnInitializeAbility`)
  (return))

(fn `PrintDebugMessage`
  (params (InString :type String))
  (if (`self.IsDebugModeOn`)
    (`KismetSystemLibrary.PrintString` null InString)
    (return)))