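; Actor component that serves as a custom Blueprint ability system for ARPG base characters, granting and activating abilities.
; On BeginPlay it caches the owning character, and granting constructs an object per ability class, stores it and initializes it with the owner and component.
; Activation finds the granted ability by class, checks CanActivateAbility, then runs it and records it as the active ability.
; Optional debug printing reports non-matching abilities during lookup.
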(event `self.ReceiveBeginPlay`
  (bind _asarpgbase_character_bp (cast `/Game/Framework/ARPGBaseCharacter_BP` (`self.GetOwner`)))
  (`/Engine/EditorBlueprintResources/StandardMacros.IsValid` _asarpgbase_character_bp
    (:`Is Valid`
      (set `self.OwnerCharacter` _asarpgbase_character_bp))))

(fn `GrantAbilitiesOfClass`
  (params (AbilitiesToGrant :type "Array of /Game/Framework/AbilitySystem/ARPGBaseAbility_BP Class Reference"))
  (locals (L_AbilityObject :type "/Game/Framework/AbilitySystem/ARPGBaseAbility_BP Object Reference"))
  (for _array_element AbilitiesToGrant
    (if (`KismetSystemLibrary.IsValidClass` _array_element)
      (bind _returnvalue (`|GenericCreateObject` _array_element))
      (`/Engine/EditorBlueprintResources/StandardMacros.IsValid` _returnvalue
        (:`Is Valid`
          (bind _output_get (set `local.L_AbilityObject` _returnvalue))
          (`KismetArrayLibrary.Array_Add` (`self.OwnerAbilities`) _output_get)
          (`/Game/Framework/AbilitySystem/ARPGBaseAbility_BP.InitializeAbility` (`local.L_AbilityObject`) (`self.OwnerCharacter`) self))))))

(fn `PrintDebugMessage`
  (params (InString :type String))
  (if (`self.IsDebugModeOn`)
    (`KismetSystemLibrary.PrintString` InString)
    (return)))

(fn `TryActivateAbilityOfClass`
  (params (AbilityToActivate :type "/Game/Framework/AbilitySystem/ARPGBaseAbility_BP Class Reference"))
  (locals (L_AbilityToActivate :type "/Game/Framework/AbilitySystem/ARPGBaseAbility_BP Object Reference"))
  (bind _l_abilitytoactivate (`local.L_AbilityToActivate`))
  (for _array_element (`self.OwnerAbilities`)
    (if (== (`GameplayStatics.GetObjectClass` _array_element) (`local.AbilityToActivate`))
      (set `local.L_AbilityToActivate` _array_element)
      (else
        (`self.PrintDebugMessage` "AbilityNotGranted"))))
  (if (`/Game/Framework/AbilitySystem/ARPGBaseAbility_BP.CanActivateAbility` _l_abilitytoactivate)
    (`/Game/Framework/AbilitySystem/ARPGBaseAbility_BP.OnActivateAbility` _l_abilitytoactivate)
    (set `self.ActiveAbility` _l_abilitytoactivate)))